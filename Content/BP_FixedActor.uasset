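; BP_FixedActor is an actor that keeps its placed location quantized for use with fixed-point vector math.
; Its construction script scales the location by Accuracy, truncates it to integers, divides in fixed-point, then sets the converted result as the actor's location.
; GetFixedLocation returns the current location converted to a fixed vector.
; The event graph holds only disabled placeholder events, so it adds no runtime behavior.
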(fn `GetFixedLocation`
  (returns (FixedLocation :type "FixedVector Structure"))
  (return (`BlueprintFixedVectorMath.VectorToFixedVector` (`self.K2_GetActorLocation`))))

(fn `UserConstructionScript`
  (bind _accuracy (`self.Accuracy`))
  (`self.K2_SetActorLocation` (`BlueprintFixedVectorMath.FixedVectorToVector` (`BlueprintFixedVectorMath.Divide` (`BlueprintFixedVectorMath.IntVectorToFixedVector` (`KismetMathLibrary.FTruncVector` (* (`self.K2_GetActorLocation`) _accuracy))) (`BlueprintFixedVectorMath.FixedToFixedVector` (`BlueprintFixedMath.IntToFixed` _accuracy))))))