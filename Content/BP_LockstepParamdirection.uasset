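; BP_LockstepParamdirection is a lockstep parameter that carries a single Direction enum value as raw bytes.
; GenBytes sizes RawData to one byte and writes Direction into it.
; ParBytes reads that byte back into an EDirection, returning false if RawData is not exactly one byte long.
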(fn `GenBytes`
  (returns (ReturnValue :type Boolean))
  (bind _rawdata (`self.RawData`))
  (`KismetArrayLibrary.Array_Resize` _rawdata 1)
  (`KismetArrayLibrary.Array_Set` _rawdata 0 (`self.Direction`))
  (return true))

(fn `ParBytes`
  (returns (ReturnValue :type Boolean))
  (if (== (`KismetArrayLibrary.Array_Length` (`self.RawData`)) 1)
    (set `self.Direction` (cast `/Game/EDirection` (`|GetArrayItem` (`self.RawData`))))
    (return true)
    (else
      (return false))))