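; Player controller that drives a cube through a LockstepManager and exposes round register and join calls, with a UMG widget holding a reference to it.
; WASD, Space and X send move, stop and return events, whose lockstep callbacks change Speed or Target.
; Each lockstep tick advances Target by Speed and records tick intervals, while frame Tick updates the manager and interpolates the cube toward Target.
; A looping timer sends void events as keep-alives.
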(event `self.ReceiveTick`
  (params (DeltaSeconds :type "Float (single-precision)"))
  (bind _lockstep (`self.Lockstep`)
    (:`then`
      (`LockstepManager.Update` _lockstep)
      (`KismetSystemLibrary.PrintString` (`KismetStringLibrary.Conv_VectorToString` (`SceneComponent.K2_GetComponentLocation` (`StaticMeshActor.StaticMeshComponent` (`self.Mesh`)))) true true (struct :`G` 0.66 :`B` 1.0 :`A` 1.0) DeltaSeconds)
      (`KismetSystemLibrary.PrintString` (`KismetStringLibrary.Conv_VectorToString` (`self.Target`)) true true (struct :`G` 0.66 :`B` 1.0 :`A` 1.0) DeltaSeconds)
      (`KismetSystemLibrary.PrintString` (`KismetStringLibrary.Conv_VectorToString` (`self.Speed`)) true true (struct :`G` 0.66 :`B` 1.0 :`A` 1.0) DeltaSeconds)
      (`self.Raw Tick Move` DeltaSeconds))
    (:`else`)))

(event `self.ReceiveBeginPlay`
  (`|ExecutionSequence`
    (:`then_0`
      (bind _returnvalue (`|CreateWidget` "/Game/UMG_S.UMG_S_C"))
      (bind _output_get (set `self.UMG` _returnvalue))
      (`UserWidget.AddToViewport` _returnvalue 0)
      (`UserWidget.AddToViewport` _output_get 0)
      (set `/Game/UMG_S.PC` self _output_get))
    (:`then_1`
      (bind _returnvalue_2 (`|GenericCreateObject` "/Script/Lockstep.LockstepManager" self))
      (bind _output_get_2 (set `self.Lockstep` _returnvalue_2))
      (set `LockstepManager.EventRegistry` "/Game/DT_LockstepEvents.DT_LockstepEvents" _output_get_2)
      (`LockstepManager.Initialization` _output_get_2)
      (`LockstepManager.BindEvent` _output_get_2 "Tick" (delegate `Lockstep Tick`))
      (add `LockstepManager.OnThrowError` _output_get_2 (delegate `Lockstep Error`))
      (`LockstepManager.BindEvent` _output_get_2 "Move" (delegate `Lockstep Move`))
      (`LockstepManager.BindEvent` _output_get_2 "Stop" (delegate `Lockstep Stop`))
      (`LockstepManager.BindEvent` _output_get_2 "Return" (delegate `Lockstep Return`))
      (`KismetSystemLibrary.K2_SetTimerDelegate` (delegate `Prevent Timeout`) 1.0 true)
      (bind _returnvalue_3 (`GameplayStatics.GetActorOfClass` "/Game/BP_Cube.BP_Cube_C"))
      (bind _output_get_3 (set `self.Mesh` _returnvalue_3))
      (set `self.Target` (`self.K2_GetActorLocation` _output_get_3)))
    (:`then_2`
      (bind _returnvalue_4 (`|GenericCreateObject` "/Script/Lockstep.LockstepParamVoid" self))
      (set `self.VoidParam` _returnvalue_4)
      (bind _returnvalue_5 (`|GenericCreateObject` "/Game/BP_LockstepParamdirection.BP_LockstepParamDirection_C" self))
      (set `self.MoveParam` _returnvalue_5))))

(event `Lockstep Tick`
  (params (Params :type "LockstepParamBase Object Reference"))
  (bind (_seconds _partialseconds) (`GameplayStatics.GetAccurateRealTime`))
  (bind _tickindex (`self.TickIndex`))
  (bind _returnvalue (+ (`KismetMathLibrary.Conv_IntToDouble` _seconds) _partialseconds))
  (bind _aslockstep_param_int_32 (cast `LockstepParamInt32` Params))
  (set `self.LastTick` (`LockstepParamInt32.Value` _aslockstep_param_int_32))
  (`|ExecutionSequence`
    (:`then_0`
      (`|ExecutionSequence`
        (:`then_0`
          (`/Engine/EditorBlueprintResources/StandardMacros.DoOnce` false :!label _label
            (:`Completed`
              (`KismetArrayLibrary.Array_Set` (`self.TickArray`) (mod _tickindex 256) (- _returnvalue (`self.LastTickTime`)) true)
              (`/Engine/EditorBlueprintResources/StandardMacros.IncrementInt` _tickindex
                (:`  `
                  (set `self.LastTickTime` _returnvalue))))))
        (:`then_1`
          (goto _label :!via `Reset`))))
    (:`then_1`
      (`self.Lockstep Tick Move`))))

(event `Lockstep Error`
  (params (FailureType :type "ELockstepError Enum" :default "Timeout"))
  (`KismetSystemLibrary.PrintString` (`|GetEnumeratorNameAsString` FailureType) true true (struct :`G` 0.66 :`B` 1.0 :`A` 1.0) 10.0))

(event `Prevent Timeout`
  (bind _lockstep (`self.Lockstep`)
    (:`then`
      (`LockstepManager.SendEvent` _lockstep "Void" (`self.VoidParam`)))
    (:`else`)))

(event `Raw Tick Move`
  (params (DeltaTime :type "Float (double-precision)"))
  (bind _mesh (`self.Mesh`))
  (`self.K2_SetActorLocation` _mesh (`KismetMathLibrary.VInterpTo` (`self.K2_GetActorLocation` _mesh) (`self.Target`) DeltaTime 15.0) false false))

(event `Lockstep Move`
  (params (Params :type "LockstepParamBase Object Reference"))
  (bind _acceleration (`self.Acceleration`))
  (bind _asbp_lockstep_param_direction (cast `/Game/BP_LockstepParamdirection` Params))
  (switch `/Game/EDirection` (`/Game/BP_LockstepParamdirection.Direction` _asbp_lockstep_param_direction)
    (:`NewEnumerator0`
      (bind _output_get (set `self.Speed` (+ (stale _output_get) (* (1.0 0.0 0.0) _acceleration)))))
    (:`NewEnumerator1`
      (bind _output_get_2 (set `self.Speed` (+ (stale _output_get_2) (* (-1.0 0.0 0.0) _acceleration)))))
    (:`NewEnumerator2`
      (bind _output_get_3 (set `self.Speed` (+ (stale _output_get_3) (* (0.0 1.0 0.0) _acceleration)))))
    (:`NewEnumerator3`
      (bind _output_get_4 (set `self.Speed` (+ (stale _output_get_4) (* (0.0 -1.0 0.0) _acceleration)))))))

(event `Lockstep Tick Move`
  (bind _moveparam (`self.MoveParam`))
  (`|ExecutionSequence`
    (:`then_0`
      (bind _output_get (set `self.Target` (+ (stale _output_get) (`self.Speed`)))))
    (:`then_1`
      (if (`self.IsInputKeyDown` "W")
        (bind _lockstep (`self.Lockstep`)
          (:`then`
            (set `/Game/BP_LockstepParamdirection.Direction` "NewEnumerator0" _moveparam)
            (`LockstepManager.SendEvent` _lockstep "Move" _moveparam))
          (:`else`))))
    (:`then_2`
      (if (`self.IsInputKeyDown` "S")
        (bind _lockstep_2 (`self.Lockstep`)
          (:`then`
            (set `/Game/BP_LockstepParamdirection.Direction` "NewEnumerator1" _moveparam)
            (`LockstepManager.SendEvent` _lockstep_2 "Move" _moveparam))
          (:`else`))))
    (:`then_3`
      (if (`self.IsInputKeyDown` "D")
        (bind _lockstep_3 (`self.Lockstep`)
          (:`then`
            (set `/Game/BP_LockstepParamdirection.Direction` "NewEnumerator2" _moveparam)
            (`LockstepManager.SendEvent` _lockstep_3 "Move" _moveparam))
          (:`else`))))
    (:`then_4`
      (if (`self.IsInputKeyDown` "A")
        (bind _lockstep_4 (`self.Lockstep`)
          (:`then`
            (set `/Game/BP_LockstepParamdirection.Direction` "NewEnumerator3" _moveparam)
            (`LockstepManager.SendEvent` _lockstep_4 "Move" _moveparam))
          (:`else`))))))

(event `Lockstep Stop`
  (params (Params :type "LockstepParamBase Object Reference"))
  (set `self.Speed` (0.0 0.0 0.0)))

(event `Key|SpaceBar`
  (params (Key :type "Key Structure"))
  (:`Pressed`
    (bind _lockstep (`self.Lockstep`)
      (:`then`
        (`LockstepManager.SendEvent` _lockstep "Stop" (`self.VoidParam`)))
      (:`else`))))

(event `Lockstep Return`
  (params (Params :type "LockstepParamBase Object Reference"))
  (set `self.Target` (0.0 0.0 0.0)))

(event `Key|X`
  (params (Key :type "Key Structure"))
  (:`Pressed`
    (bind _lockstep (`self.Lockstep`)
      (:`then`
        (`LockstepManager.SendEvent` _lockstep "Return" (`self.VoidParam`)))
      (:`else`))))

(fn `Join Round`
  (params (IP :type String) (Port :type Integer) (RoundName :type String) (Password :type String))
  (returns (ReturnValue :type "ELockstepReturn Enum"))
  (bind _returnvalue (`LockstepManager.JoinRound` (`self.Lockstep`) IP Port RoundName Password))
  (return _returnvalue))

(fn `Register Round`
  (params (IP :type String) (Port :type Integer) (RoundName :type String) (Password :type String))
  (returns (ReturnValue :type "ELockstepReturn Enum"))
  (bind _returnvalue (`LockstepManager.RegisterRound` (`self.Lockstep`) IP Port RoundName Password))
  (return _returnvalue))

(fn `UserConstructionScript`)